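; Interactable actor Blueprint that changes the color of its Cube mesh while it has focus.
; On BeginPlay it creates a dynamic material instance on the cube and caches the original "Color" parameter value.
; StartFocus sets that parameter to StartColour, and EndFocus restores the cached default.
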(event `self.ReceiveBeginPlay`
  (bind _returnvalue (`PrimitiveComponent.CreateDynamicMaterialInstance` (`self.Cube`) 0 null "None"))
  (bind _output_get (set `self.Material Instance` _returnvalue))
  (bind _returnvalue_2 (`MaterialInstanceDynamic.K2_GetVectorParameterValue` _output_get "Color"))
  (set `self.Default Color` _returnvalue_2))

(event `self.StartFocus`
  (`MaterialInstanceDynamic.SetVectorParameterValue` (`self.Material Instance`) "Color" (`self.StartColour`)))

(event `self.EndFocus`
  (`MaterialInstanceDynamic.SetVectorParameterValue` (`self.Material Instance`) "Color" (`self.Default Color`)))

(fn `UserConstructionScript`)