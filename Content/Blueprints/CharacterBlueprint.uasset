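; Player character Blueprint that manages the crosshair and HUD and triggers interactions on overlap.
; BeginPlay saves its transform as the game mode's spawn point, while Tick creates both widgets if missing outside the MainMenu level.
; Mesh overlaps message the other actor, damage refreshes the HUD power display, and cursor focus events swap the crosshair texture.
; Forward tracing defers to the parent class, leaving the Blueprint line trace unconnected.
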(event `self.ReceiveBeginPlay`
  (bind _ascharacter_game_mode_base (cast `/Game/Blueprints/Character_GameModeBase` (`GameplayStatics.GetGameMode`)))
  (set `/Game/Blueprints/Character_GameModeBase.SpawnTransform` (`self.GetTransform`) _ascharacter_game_mode_base))

(event `self.ReceiveTick`
  (params (DeltaSeconds :type "Float (single-precision)"))
  (bind _returnvalue (`GameplayStatics.GetCurrentLevelName` true))
  (if (not (`KismetStringLibrary.EqualEqual_StrStr` _returnvalue "MainMenu"))
    (`/Engine/EditorBlueprintResources/StandardMacros.IsValid` (`self.CrosshairRef`)
      (:`Is Valid`
        _)
      (:`Is Not Valid`
        (bind _returnvalue_2 (`|CreateWidget` "/Game/Blueprints/UI/Crosshair.Crosshair_C"))
        (bind _output_get (set `self.CrosshairRef` _returnvalue_2))
        (`UserWidget.AddToViewport` _output_get 0)))
    (`/Engine/EditorBlueprintResources/StandardMacros.IsValid` (`self.HUDReference`)
      (:`Is Not Valid`
        (bind _returnvalue_3 (`|CreateWidget` "/Game/Blueprints/UI/HUD.HUD_C"))
        (bind _output_get_2 (set `self.HUDReference` _returnvalue_3))
        (`UserWidget.AddToViewport` _output_get_2 0)))))

(event `InputAction|Interact`
  (params (Key :type "Key Structure"))
  ;[1 1 1] Connect the LineTraceByChannel and InputAction Interact blocks to implement this function. This is disabled as it is already done using C++.
)

(event `self.CharacterMesh.OnComponentBeginOverlap`
  (params (OverlappedComponent :type "PrimitiveComponent Object Reference") (OtherActor :type "Actor Object Reference") (OtherComp :type "PrimitiveComponent Object Reference") (OtherBodyIndex :type Integer) (bFromSweep :type Boolean) (SweepResult :type "HitResult Structure (by ref)"))
  (message `InteractInterface.OnInteract` OtherActor self))

(event `self.TraceForward`
  (`parent.TraceForward`))

(event `self.ReceiveAnyDamage`
  (params (Damage :type "Float (single-precision)") (DamageType :type "DamageType Object Reference") (InstigatedBy :type "Controller Object Reference") (DamageCauser :type "Actor Object Reference"))
  (bind _power (`self.Power`))
  (`/Engine/EditorBlueprintResources/StandardMacros.IsValid` (`self.HUDReference`)
    (:`Is Valid`
      (`/Game/Blueprints/UI/HUD.UpdatePower` (`self.HUDReference`) (`PowerComponent.Power` _power) (`PowerComponent.MaxPower` _power)))))

(event `self.CursorFocusStart`
  (`Image.SetBrushFromTexture` (`/Game/Blueprints/UI/Crosshair.Image_229` (`self.CrosshairRef`)) "/Game/Images/CrosshairGreen.CrosshairGreen" false))

(event `self.CursorFocusStop`
  (`Image.SetBrushFromTexture` (`/Game/Blueprints/UI/Crosshair.Image_229` (`self.CrosshairRef`)) "/Game/Images/Crosshair.Crosshair" false))

(fn `UserConstructionScript`)